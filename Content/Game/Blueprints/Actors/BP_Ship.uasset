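; BP_Ship is a ship actor that procedurally animates its mesh with a repeating rocking rotation.
; A random startup delay on BeginPlay keeps multiple ships out of sync.
; The ShipAnimation timeline scales one RotationAmount track by random pitch and roll multipliers, leaving yaw unchanged.
; Each time the timeline finishes, it picks new multipliers within the min/max ranges and replays, so every cycle varies.
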(event `self.ReceiveBeginPlay`
  (bind _shipmesh (`self.ShipMesh`))
  (bind _shipmesh_2 (`self.ShipMesh`))
  (bind (_relativerotation_roll _relativerotation_pitch _relativerotation_yaw) (`KismetMathLibrary.BreakRotator` (`SceneComponent.RelativeRotation` _shipmesh)))
  (bind (_relativerotation_roll_2 _relativerotation_pitch_2 _relativerotation_yaw_2) (`KismetMathLibrary.BreakRotator` (`SceneComponent.RelativeRotation` _shipmesh_2)))
  ;[1 1 1] Delay to make the ships out of sync even more
  (`KismetSystemLibrary.Delay` (`KismetMathLibrary.RandomFloatInRange` 2.0 9.0))
  (set `self.Y Rotation Multiplier Current` (`KismetMathLibrary.RandomFloatInRange` (`self.Y Rotation Multiplier Min`) (`self.Y Rotation Multiplier Max`)) :!label _label)
  (set `self.X Rotation Multiplier Current` (`KismetMathLibrary.RandomFloatInRange` (`self.X Rotation Multiplier Min`) (`self.X Rotation Multiplier Max`)))
  (bind (_direction _rotation_amount) (`Timeline|ShipAnimation` :!via `PlayFromStart`)
    (:`Update`
      ;[1 1 1] Rotate Ship Around Y
      (`SceneComponent.K2_SetRelativeRotation` _shipmesh_2 (`KismetMathLibrary.MakeRotator` _relativerotation_roll_2 (* _rotation_amount (`self.Y Rotation Multiplier Current`)) _relativerotation_yaw_2) false false)
      ;[1 1 1] Set Rotation X
      (`SceneComponent.K2_SetRelativeRotation` _shipmesh (`KismetMathLibrary.MakeRotator` (* _rotation_amount (`self.X Rotation Multiplier Current`)) _relativerotation_pitch _relativerotation_yaw) false false))
    (:`Finished`
      (goto _label))))

(fn `UserConstructionScript`)